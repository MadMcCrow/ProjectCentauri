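; Player controller for a ship-building mode that spawns a spaceship pawn and lets the player attach parts to it.
; BeginPlay creates the mode menu and a hidden attach-options menu, while SetBuildingBP spawns the ship and aims the CameraPawn at it.
; In Building state, selecting an AttachComponent reveals the options and refocuses the camera on the ship.
; AddItem messages the component's owning SpaceActor to attach the chosen class there.
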(event Custom|AddItem
  (params (Class%20to%20spawn :type Space%20Actor%20Class%20Reference))
  (bind _asattach_component (Utilities|Casting|CastToAttachComponent (Class|SpacePlayerController|GetSelectedComponentBP)))
  (bind _asspace_actor (Utilities|Casting|CastToSpaceActor (Components|GetOwner (Class|SpacePlayerController|GetSelectedComponentBP))))
  (Class|ChildInterface|AddAttachSpaceActorBP(Message) _asspace_actor Class%20to%20spawn _asattach_component))

(event EventSetBuildingBP
  (bind _returnvalue (Pawn|GetControlledPawn))
  (bind _returnvalue_2 (Game|SpawnActorfromClass "/Game/Actors/Blueprint/SpaceShipPawn_BP.SpaceShipPawn_BP_C" (Math|Transform|MakeTransform (.Location (Math|Transform|BreakTransform (Transformation|GetActorTransform)))) "AlwaysSpawn" _returnvalue _returnvalue))
  (Variables|Default|SetSpaceship _returnvalue_2)
  (bind _ascamera_pawn (Utilities|Casting|CastToCameraPawn _returnvalue))
  (bind _output_get (Variables|Default|SetCameraPawn _ascamera_pawn))
  (Class|CameraPawn|SetLookatObjectBP _output_get (Variables|Default|GetSpaceship) 1e+02))

(event EventTick
  (params (DeltaSeconds :type Float%20%28single-precision%29)))

(event EventBeginPlay
  (Utilities|FlowControl|Sequence
    (:then_0
      (bind _returnvalue (UserInterface|CreateWidget "/Game/UI/UI_Mode_Menu.UI_Mode_Menu_C" self))
      (bind _returnvalue_2 (UserInterface|Viewport|AddtoPlayerScreen _returnvalue))
      (Variables|Default|SetbShowMouseCursor _returnvalue_2))
    (:then_1
      (bind _returnvalue_3 (UserInterface|CreateWidget "/Game/UI/Build/UI_AttachOptions.UI_AttachOptions_C" self))
      (bind _output_get (Variables|Default|SetBuildMenu _returnvalue_3))
      (UserInterface|Viewport|AddtoPlayerScreen _output_get)
      (Widget|SetVisibility (Variables|Default|GetBuildMenu) "Hidden"))))

(event EventOnSelectBP
  (bind _buildmenu (Variables|Default|GetBuildMenu))
  (switch Utilities|FlowControl|Switch|SwitchonEControllerStateEnum "CSE_Build"
    (:CSE_Build
      (Utilities|FlowControl|Sequence
        (:then_0
          (bind _asattach_component (Utilities|Casting|CastToAttachComponent (Class|SpacePlayerController|GetSelectedComponentBP))
            (:then
              (Widget|SetVisibility _buildmenu "Visible")
              (Class|CameraPawn|SetLookatObjectBP (Variables|Default|GetCameraPawn) (Variables|Default|GetSpaceship) 1e+02))
            (:CastFailed
              (Widget|SetVisibility _buildmenu "Hidden"))))))))

(fn ConstructionScript)